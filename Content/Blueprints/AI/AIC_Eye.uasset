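; AIC_Eye is the AI controller for BP_Enemy_Eye, steering the enemy toward a target player.
; It caches the possessed Eye on possession and receives its target through the SetTargetPlayer event.
; Each tick, while both are valid, it passes the look-at direction to the target into the Eye's MoveToward at full scale.
; The chase follows a straight line, with no navmesh pathing or behavior tree.
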(event `self.ReceivePossess`
  (params (PossessedPawn :type "Pawn Object Reference"))
  (bind _asbp_enemy_eye (cast `/Game/Blueprints/Characters/Enemies/Lecture/Eye/BP_Enemy_Eye` PossessedPawn))
  (set `self.Owning Eye` _asbp_enemy_eye))

(event `self.ReceiveTick`
  (params (DeltaSeconds :type "Float (single-precision)"))
  (`parent.ReceiveTick` DeltaSeconds)
  (`/Engine/EditorBlueprintResources/StandardMacros.IsValid` (`self.Owning Eye`)
    (:`Is Valid`
      (`/Engine/EditorBlueprintResources/StandardMacros.IsValid` (`self.Target Player`)
        (:`Is Valid`
          (`/Game/Blueprints/Characters/Enemies/Lecture/Eye/BP_Enemy_Eye.MoveToward` (`self.Owning Eye`) (`KismetMathLibrary.GetForwardVector` (`KismetMathLibrary.FindLookAtRotation` (`self.K2_GetActorLocation` (`self.Owning Eye`)) (`self.K2_GetActorLocation` (`self.Target Player`)))) 1.0))))))

(event `Set TargetPlayer`
  (params (`Target Player` :type "Pawn Object Reference"))
  ;[0 0 0] Set Target(Player)
  (set `self.Target Player` `Target Player`))

(fn `UserConstructionScript`
  (`parent.UserConstructionScript`))