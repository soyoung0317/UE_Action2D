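; AI controller for the slime enemy that keeps it moving and steers it toward a detected player.
; On possess it caches the slime pawn, and TargetSetting stores the pawn passed to it as the target, with no clearing logic.
; Each tick calls the slime's MoveTo along MonsterToPlayerVector, or straight forward without a target.
; The look-at forward vector in MonsterToPlayerVector appears unconnected to any output.
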(event `self.ReceivePossess`
  (params (PossessedPawn :type "Pawn Object Reference"))
  ;[0 0 0] Initializer : Owner 설정
  (bind _asbp_enemy_slime (cast `/Game/Blueprints/Characters/Enemies/Slime/BP_Enemy_Slime` PossessedPawn))
  (set `self.Owning Slime` _asbp_enemy_slime))

(event `self.ReceiveTick`
  (params (DeltaSeconds :type "Float (single-precision)"))
  ;[0 0 0] Tick : 플레이어 포착되었다면 플레이어 방향쪽으로 이동 함수 호출 및 회전
  (`parent.ReceiveTick` DeltaSeconds)
  (`/Engine/EditorBlueprintResources/StandardMacros.IsValid` (`self.Owning Slime`)
    (:`Is Valid`
      (`/Engine/EditorBlueprintResources/StandardMacros.IsValid` (`self.Target Player`)
        (:`Is Valid`
          (`/Game/Blueprints/Characters/Enemies/Slime/BP_Enemy_Slime.Move To` (`self.Owning Slime`) (`KismetMathLibrary.GetForwardVector` (`KismetMathLibrary.FindLookAtRotation` (`self.K2_GetActorLocation` (`self.Owning Slime`)) (`self.K2_GetActorLocation` (`self.Target Player`)))) 1.0))
        (:`Is Not Valid`
          (`/Game/Blueprints/Characters/Enemies/Slime/BP_Enemy_Slime.Move To` (`self.Owning Slime`) (`self.GetActorForwardVector` (`self.Owning Slime`)) 1.0))))))

(event `Target Setting`
  (params (`Overlap Pawn` :type "Pawn Object Reference"))
  ;[0 0 0] 목표를 포착했다
  (set `self.Target Player` `Overlap Pawn`))

(fn `UserConstructionScript`
  (`parent.UserConstructionScript`))