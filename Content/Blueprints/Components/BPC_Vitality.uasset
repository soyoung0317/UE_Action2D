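; BPC_Vitality is a health component that tracks an object's current health and defeated state.
; On BeginPlay it sets CurrentHealth to MaxHealth.
; ReceiveDamage, intended to be called from the owning object's AnyDamage event, subtracts damage, clamps health between zero and MaxHealth, and sets IsDefeated once health reaches zero.
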(event `self.ReceiveBeginPlay`
  ;[0 0 0] Event BeginPlay : 초기 현재hp값 max로 설정
  (set `self.CurrentHealth` (`self.MaxHealth`)))

(fn `Receive Damage`
  (params (DaMAGE :type "Float (double-precision)"))
  ;[0 0 0] Function : 객체에서 Event AnyDamage함수 호출시 Health 차감
  (set `self.CurrentHealth` (`KismetMathLibrary.FClamp` (- (`self.CurrentHealth`) DaMAGE) 0.0 (`self.MaxHealth`)))
  (if (<= (`self.CurrentHealth`) 0.0)
    (set `self.IsDefeated` true)))