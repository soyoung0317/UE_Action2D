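; GM_Action is the game mode that runs the quest flow, HUD, cutscene hooks and player respawning.
; After a delayed intro that spawns a UFO, Tick polls a quest-progress state machine, advancing some dialogue steps on the player's E press through DoOnce gates.
; External events can set progress, update the cat quest counter, trigger cutscene UI and spawn boss fires.
; RespawnPlayer spawns and possesses a new pawn at the active checkpoint, falling back to PlayerStart.
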(event `self.ReceiveBeginPlay`
  ;[0 0 0] Comment
  (`|ExecutionSequence`
    (:`then_0`
      (bind _returnvalue (`GameplayStatics.GetActorOfClass` "/Script/Engine.PlayerStart")) ; 액터 시작지점
      (set `self.PlayerStart` _returnvalue)
      (set `self.GM_Quest Progress` "NewEnumerator0") ; 퀘스트 초기화
      (set `self.Is Controlling` true))
    (:`then_1`
      (bind _returnvalue_2 (`|CreateWidget` "/Game/Widgets/WBP_HUD.WBP_HUD_C" (`GameplayStatics.GetPlayerController` 0))) ; 기본 플레이어 체력 위젯
      (bind _output_get (set `self.HUD widget` _returnvalue_2))
      (`UserWidget.AddToViewport` _output_get 0))
    (:`then_2`
      (bind _asbp_player (cast `/Game/Blueprints/Characters/Player/BP_Player` (`GameplayStatics.GetPlayerCharacter` 0))) ; 플레이어 받아오기
      (set `self.BP Player` _asbp_player))))

(event `Control Quest`
  ;[0.3417 1 0.04393] Quest Controll
  (switch `/Game/Blueprints/Enums/E_QuestProgress` (`self.GM_Quest Progress`)
    (:`NewEnumerator1`
      (`/Engine/EditorBlueprintResources/StandardMacros.DoOnce` false
        (:`Completed`
          (bind _returnvalue (`|CreateWidget` "/Game/Widgets/Quest/WBP_Quest0_Talk.WBP_Quest0_Talk_C" (`GameplayStatics.GetPlayerController` 0))) ; 위젯 만들고 띄우기
          (bind _output_get (set `self.Quest Widget` _returnvalue))
          (`UserWidget.AddToViewport` _output_get 0)
          (set `/Game/Widgets/Quest/WBP_Quest0_Talk.widget Current Quest Progress` "NewEnumerator2" _output_get)
          (set `self.GM_Quest Progress` "NewEnumerator2"))))
    (:`NewEnumerator2`
      (if (`/Game/Blueprints/Characters/Player/BP_Player.Is Pressed E` (`self.BP Player`))
        (`/Engine/EditorBlueprintResources/StandardMacros.DoOnce` false
          (:`Completed`
            (set `/Game/Blueprints/Characters/Player/BP_Player.Is Pressed E` false (`self.BP Player`))
            (set `/Game/Widgets/Quest/WBP_Quest0_Talk.widget Current Quest Progress` "NewEnumerator3" (`self.Quest Widget`))
            (set `self.GM_Quest Progress` "NewEnumerator3")))))
    (:`NewEnumerator3`)
    (:`NewEnumerator4`
      (if (`/Game/Blueprints/Characters/Player/BP_Player.Is Pressed E` (`self.BP Player`))
        (`/Engine/EditorBlueprintResources/StandardMacros.DoOnce` false
          (:`Completed`
            (set `/Game/Blueprints/Characters/Player/BP_Player.Is Pressed E` false (`self.BP Player`))
            (set `/Game/Widgets/Quest/WBP_Quest0_Talk.widget Current Quest Progress` "NewEnumerator5" (`self.Quest Widget`))
            (set `self.GM_Quest Progress` "NewEnumerator5")))))
    (:`NewEnumerator5`)
    (:`NewEnumerator6`
      (if (`/Game/Blueprints/Characters/Player/BP_Player.Is Pressed E` (`self.BP Player`))
        (`/Engine/EditorBlueprintResources/StandardMacros.DoOnce` false
          (:`Completed`
            (set `/Game/Blueprints/Characters/Player/BP_Player.Is Pressed E` false (`self.BP Player`))
            (set `/Game/Widgets/Quest/WBP_Quest0_Talk.widget Current Quest Progress` "NewEnumerator7" (`self.Quest Widget`))
            (set `self.GM_Quest Progress` "NewEnumerator7")))))
    (:`NewEnumerator8`
      (`/Engine/EditorBlueprintResources/StandardMacros.DoOnce` false
        (:`Completed`
          (`Widget.SetVisibility` (`/Game/Widgets/WBP_HUD.WBP_QuestWindow` (`self.HUD widget`)) "Visible")
          (`UserWidget.AddToViewport` (`/Game/Widgets/WBP_HUD.WBP_QuestWindow` (`self.HUD widget`)) 0))))))

(event `self.ReceiveTick`
  (params (DeltaSeconds :type "Float (single-precision)"))
  ;[0 0 0] Comment
  (if (`self.Is Controlling`)
    (if (`self.bGameStart`)
      (`self.Control Quest`) ; 퀘스트 컨트롤
      (else
        (`KismetSystemLibrary.Delay` (`self.Game StartDelay`))
        (`/Engine/EditorBlueprintResources/StandardMacros.DoOnce` false
          (:`Completed`
            (`GameplayStatics.PlaySound2D` "/Game/Audio/Background/Gentle_Breeze_Cue.Gentle_Breeze_Cue" 1.0 1.0 0.0 null null)
            (`|SpawnActorFromClass` "/Game/Blueprints/Props/BP_Props_UFO.BP_Props_UFO_C" (`KismetMathLibrary.MakeTransform` (998.0 -0.1 -1630.0)) "Undefined" "MultiplyWithRoot" null null)
            (set `self.bGameStart` true)))))))

(event `GM_Change Quest Progress`
  (params (`New Progress` :type "/Game/Blueprints/Enums/E_QuestProgress Enum" :default "NewEnumerator0"))
  ;[0 0 0] Quest 진행에 필요
  (set `self.GM_Quest Progress` `New Progress`))

(event `Quest FindCat Update`
  ;[0 0 0] Quest Controll - 좌상단 퀘스트 컨트롤
  (`/Game/Widgets/Quest/WBP_QuestWindow.Add Cat Cnt` (`/Game/Widgets/WBP_HUD.WBP_QuestWindow` (`self.HUD widget`))))

(event `First Cutscene start`
  ;[0 0 0] 컷신 시작하게하기
  (`/Game/Widgets/WBP_HUD.First Cutscene Start` (`self.HUD widget`)))

(event `Final Cutscene`
  (`Widget.SetVisibility` (`self.HUD widget`) "Hidden")
  (bind _returnvalue (`|CreateWidget` "/Game/Widgets/WBP_Final.WBP_Final_C" (`GameplayStatics.GetPlayerController` 0))) ; 기본 플레이어 체력 위젯
  (`UserWidget.AddToViewport` _returnvalue 0))

(event `First Cutscene End`
  ;[1 1 1] Comment
  (`/Engine/EditorBlueprintResources/StandardMacros.IsValid` (`self.BP Player`)
    (:`Is Valid`
      (`/Game/Blueprints/Characters/Player/BP_Player.Set Rendering` (`self.BP Player`) false))))

(event `Boss Fire`
  ;[1 1 1] q
  (bind _returnvalue (`|SpawnActorFromClass` "/Game/Blueprints/Effect/BP_Effect_BossFire.BP_Effect_BossFire_C" (`KismetMathLibrary.MakeTransform` (10020.5 0.1 -1146.5) (struct) (1.5 1.5 1.5)) "AlwaysSpawn" "MultiplyWithRoot" null null))
  (set `self.Left Fire` _returnvalue)
  (bind _returnvalue_2 (`|SpawnActorFromClass` "/Game/Blueprints/Effect/BP_Effect_BossFire.BP_Effect_BossFire_C" (`KismetMathLibrary.MakeTransform` (10467.0 0.1 -1146.5) (struct) (1.5 1.5 1.5)) "AlwaysSpawn" "MultiplyWithRoot" null null))
  (bind _output_get (set `self.Right Fire` _returnvalue_2))
  (set `/Game/Blueprints/Effect/BP_Effect_BossFire.Is Portal Control` true _output_get))

(fn `Progressing`
  (params (`WBP Object` :type "/Game/Widgets/Quest/WBP_Quest0_Talk Object Reference") (`Current Progress` :type "/Game/Blueprints/Enums/E_QuestProgress Enum" :default "NewEnumerator0"))
  (set `/Game/Widgets/Quest/WBP_Quest0_Talk.widget Current Quest Progress` (cast `/Game/Blueprints/Enums/E_QuestProgress` (+ `Current Progress` 1)) `WBP Object`))

(fn `Respawn Player`
  (bind (_returnvalue_location _returnvalue_rotation) (`KismetMathLibrary.BreakTransform` (`self.GetTransform` (`self.PlayerStart`))))
  (bind (_returnvalue_location_2 _returnvalue_rotation_2) (`KismetMathLibrary.BreakTransform` (`SceneComponent.K2_GetComponentToWorld` (`/Game/Blueprints/Trigger/BP_Checkpoint.Scene` (`self.ActiveCheckpoint`)))))
  (`/Engine/EditorBlueprintResources/StandardMacros.IsValid` (`self.ActiveCheckpoint`)
    (:`Is Valid`
      (bind _returnvalue (`|SpawnActorFromClass` (`self.DefaultPawnClass`) (`KismetMathLibrary.MakeTransform` _returnvalue_location_2 _returnvalue_rotation_2) "AlwaysSpawn" "MultiplyWithRoot" null null)) ; 체크포인트 리스폰
      (`Controller.Possess` (`GameplayStatics.GetPlayerController` 0) _returnvalue) ; 인자로 들어온 Pawn클래스가 컨트롤러 및 카메라를 갖게된다.
      (`GameplayStatics.PlaySound2D` "/Game/Audio/SFX/Respawn_Player_Cue.Respawn_Player_Cue" 1.0 1.0 0.0 null null))
    (:`Is Not Valid`
      (bind _returnvalue_2 (`|SpawnActorFromClass` (`self.DefaultPawnClass`) (`KismetMathLibrary.MakeTransform` _returnvalue_location _returnvalue_rotation) "AlwaysSpawn" "MultiplyWithRoot" null null)) ; 처음 시작지점 리스폰
      (`Controller.Possess` (`GameplayStatics.GetPlayerController` 0) _returnvalue_2) ; 인자로 들어온 Pawn클래스가 컨트롤러 및 카메라를 갖게된다.
      (`GameplayStatics.PlaySound2D` "/Game/Audio/SFX/Respawn_Player_Cue.Respawn_Player_Cue" 1.0 1.0 0.0 null null))))

(fn `UserConstructionScript`)