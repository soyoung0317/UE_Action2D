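; BP_Effect_BossFire is a boss fire effect that plays Paper2D burning flipbooks and can open a portal.
; Boolean phase flags advanced by OnFinishedPlaying move it from a start animation to a single loop pass, then to continuous looping.
; When IsPortalControl is set, BP_Effect_Portal spawns at a hard-coded location as continuous looping begins.
; The end-effect event is an empty stub, and debug prints remain.
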(event `self.ReceiveBeginPlay`
  (`parent.ReceiveBeginPlay`)
  (set `self.Is Fire Start` true)
  (`self.play start effect`))

(event `self.ReceiveTick`
  (params (DeltaSeconds :type "Float (single-precision)"))
  (`parent.ReceiveTick` DeltaSeconds))

(event `play start effect`
  ;[0 0 0] Start Effect
  (`PaperFlipbookComponent.SetFlipbook` (`self.PaperFlipbook`) "/Game/PaperAssets/Effect/Flipbook/burning_start_4.burning_start_4")
  (`PaperFlipbookComponent.SetLooping` (`self.PaperFlipbook`) false))

(event `play loop effect`
  ;[0 0 0] Loop Effect
  (if (`self.Is Fire LoopLoop`)
    (`PaperFlipbookComponent.SetFlipbook` (`self.PaperFlipbook`) "/Game/PaperAssets/Effect/Flipbook/burning_loop_4.burning_loop_4")
    (`PaperFlipbookComponent.SetLooping` (`self.PaperFlipbook`) true)
    (`PaperFlipbookComponent.PlayFromStart` (`self.PaperFlipbook`))
    (else
      (`PaperFlipbookComponent.SetFlipbook` (`self.PaperFlipbook`) "/Game/PaperAssets/Effect/Flipbook/burning_loop_4.burning_loop_4")
      (`PaperFlipbookComponent.SetLooping` (`self.PaperFlipbook`) false)
      (`PaperFlipbookComponent.PlayFromStart` (`self.PaperFlipbook`)))))

(event `Play Portal`
  (`|SpawnActorFromClass` "/Game/Blueprints/Effect/BP_Effect_Portal.BP_Effect_Portal_C" (`KismetMathLibrary.MakeTransform` (10361.5 0.12 -1180.0)) "AlwaysSpawn" "MultiplyWithRoot" null null))

(event `Play End Effect`)

(event `self.PaperFlipbook.OnFinishedPlaying`
  ;[0 0 0] Comment
  (if (`self.Is Fire Start`)
    (set `self.Is Fire Start` false)
    (set `self.Is Fire Loop` true)
    (`self.play loop effect`)
    (elif (`self.Is Fire Loop`)
      (if (`self.Is Fire LoopLoop`)
        (set `self.Is Fire Loop` false)
        (set `self.Is Fire End` true)
        (`KismetSystemLibrary.PrintString` "B")
        (else
          (set `self.Is Fire LoopLoop` true)
          (if (`self.Is Portal Control`)
            (`self.Play Portal`)
            (`self.play loop effect`)
            (`KismetSystemLibrary.PrintString` "A")
            (else
              (`self.play loop effect`)))))
      (elif (`self.Is Fire End`)
        (set `self.Is Fire End` false)
        (`self.Play End Effect`)))))

(fn `UserConstructionScript`
  (`parent.UserConstructionScript`))