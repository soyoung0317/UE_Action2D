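; Falling leaves effect actor that drifts downward and repeats its fall in a loop.
; On BeginPlay it picks a random move direction with a downward Z component and stores its start location.
; Each Tick it offsets itself along that fixed direction, scaled by delta time, and accumulates age.
; When age reaches LifeTime it snaps back to the start location and resets age, keeping the same direction.
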(event `self.ReceiveBeginPlay`
  ;[0 0 0] 초기 랜덤으로 움직일 Direction 받기
  (`parent.ReceiveBeginPlay`)
  (set `self.MoveDirection` (`KismetMathLibrary.MakeVector` (`KismetMathLibrary.RandomFloatInRange` -50.0 100.0) (`KismetMathLibrary.RandomFloatInRange` -0.5 1.0) (`KismetMathLibrary.RandomFloatInRange` -80.0 -100.0)))
  (set `self.StartPos` (`self.K2_GetActorLocation`)) ; 초기 위치 저장
)

(event `self.ReceiveTick`
  (params (DeltaSeconds :type "Float (single-precision)"))
  (`parent.ReceiveTick` DeltaSeconds)
  ;[0 0 0] 움직임 구현
  (`self.K2_AddActorWorldOffset` (* (`GameplayStatics.GetWorldDeltaSeconds`) (`self.MoveDirection`))) ; 랜덤D로 움직임 구현
  ;[0 0 0] 위치 반복 구현
  (set `self.Age` (+ (`GameplayStatics.GetWorldDeltaSeconds`) (`self.Age`)))
  (if (>= (`self.Age`) (`self.LifeTime`))
    (`self.K2_SetActorLocation` (`self.StartPos`))
    (set `self.Age` 0.0)))

(fn `UserConstructionScript`
  (`parent.UserConstructionScript`))