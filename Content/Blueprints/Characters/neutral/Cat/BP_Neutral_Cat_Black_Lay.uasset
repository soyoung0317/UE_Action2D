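; Neutral black cat character, animated with Paper2D flipbooks, that lies down when the player walks into its trigger.
; The overlap sets a lay flag, which Tick checks through a DoOnce gate to play the laying flipbook once, without looping.
; That flipbook's finished event switches the sprite to the resting flipbook, then to the wake-up flipbook after a short delay.
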(event `self.ReceiveTick`
  (params (DeltaSeconds :type "Float (single-precision)"))
  (`parent.ReceiveTick` DeltaSeconds)
  (`self.Behavior Laying`))

(event `Behavior Laying`
  (if (`self.Is lay`)
    (`/Engine/EditorBlueprintResources/StandardMacros.DoOnce` false
      (:`Completed`
        (`PaperFlipbookComponent.SetFlipbook` (`self.Sprite`) "/Game/PaperAssets/Characters/Neutral/Flipbook/Cat_Black_Laying.Cat_Black_Laying")
        (`PaperFlipbookComponent.SetLooping` (`self.Sprite`) false)
        (`PaperFlipbookComponent.PlayFromStart` (`self.Sprite`))
        (add `PaperFlipbookComponent.OnFinishedPlaying` (`self.Sprite`) (delegate `OnFinishedPlaying_Event`))))))

(event `OnFinishedPlaying_Event`
  (`PaperFlipbookComponent.SetFlipbook` (`self.Sprite`) "/Game/PaperAssets/Characters/Neutral/Flipbook/Cat_Black_KeepLay.Cat_Black_KeepLay")
  (`KismetSystemLibrary.Delay` 1.5)
  (`PaperFlipbookComponent.SetFlipbook` (`self.Sprite`) "/Game/PaperAssets/Characters/Neutral/Flipbook/Cat_Black_Wakeup.Cat_Black_Wakeup"))

(event `self.Trigger.OnComponentBeginOverlap`
  (params (OverlappedComponent :type "PrimitiveComponent Object Reference") (OtherActor :type "Actor Object Reference") (OtherComp :type "PrimitiveComponent Object Reference") (OtherBodyIndex :type Integer) (bFromSweep :type Boolean) (SweepResult :type "HitResult Structure (by ref)"))
  (cast `/Game/Blueprints/Characters/Player/BP_Player` OtherActor)
  (set `self.Is lay` true))

(fn `UserConstructionScript`
  (`parent.UserConstructionScript`))