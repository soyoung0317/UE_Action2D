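; BP_Neutral_MissingCat is a neutral missing-cat character that the player can find and collect by pressing E.
; On BeginPlay it spawns a half-scale heart emote effect at its Scene component's transform.
; Trigger overlaps store or clear the player reference, while Tick polls the player's IsPressedE flag during overlap.
; A single press notifies BP_Player through OverlapWithMissingCat, resets the flag and destroys the cat.
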(event `self.ReceiveBeginPlay`
  (bind _scene (`self.Scene`))
  (`parent.ReceiveBeginPlay`)
  (`|SpawnActorFromClass` "/Game/Blueprints/Effect/BP_Effect_EmoHeart.BP_Effect_EmoHeart_C" (`KismetMathLibrary.MakeTransform` (`SceneComponent.K2_GetComponentLocation` _scene) (`SceneComponent.K2_GetComponentRotation` _scene) (0.5 0.5 0.5)) "Undefined" "MultiplyWithRoot" null null))

(event `self.ReceiveTick`
  (params (DeltaSeconds :type "Float (single-precision)"))
  (`parent.ReceiveTick` DeltaSeconds)
  (if (`self.Is overlap MissingCat`)
    (if (`/Game/Blueprints/Characters/Player/BP_Player.Is Pressed E` (`self.Player Ref`))
      (`/Engine/EditorBlueprintResources/StandardMacros.DoOnce` false
        (:`Completed`
          (`/Game/Blueprints/Characters/Player/BP_Player.Overlap With Missing Cat` (`self.Player Ref`))
          (set `/Game/Blueprints/Characters/Player/BP_Player.Is Pressed E` false (`self.Player Ref`))
          (`self.K2_DestroyActor`))))))

(event `self.Trigger.OnComponentBeginOverlap`
  (params (OverlappedComponent :type "PrimitiveComponent Object Reference") (OtherActor :type "Actor Object Reference") (OtherComp :type "PrimitiveComponent Object Reference") (OtherBodyIndex :type Integer) (bFromSweep :type Boolean) (SweepResult :type "HitResult Structure (by ref)"))
  (bind _asbp_player (cast `/Game/Blueprints/Characters/Player/BP_Player` OtherActor))
  (set `self.Player Ref` _asbp_player)
  (set `self.Is overlap MissingCat` true))

(event `self.Trigger.OnComponentEndOverlap`
  (params (OverlappedComponent :type "PrimitiveComponent Object Reference") (OtherActor :type "Actor Object Reference") (OtherComp :type "PrimitiveComponent Object Reference") (OtherBodyIndex :type Integer))
  (cast `/Game/Blueprints/Characters/Player/BP_Player` OtherActor)
  (set `self.Player Ref` null)
  (set `self.Is overlap MissingCat` false))

(fn `UserConstructionScript`
  (`parent.UserConstructionScript`))