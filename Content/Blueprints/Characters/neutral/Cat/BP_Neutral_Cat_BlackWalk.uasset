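; Neutral black cat character Blueprint that randomly idles, meows, stretches or walks.
; BehaviorLoop re-rolls a random value whenever IsFinished is set, then maps its range, weighted toward idle, to a sprite flipbook or the IsWalking flag, calling itself after each branch.
; MoveForward applies movement input along the actor's forward vector, and WallDetector overlaps call TrunCharacter to turn the cat.
; BeginPlay, Tick and construction defer to the parent class.
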(event `self.ReceiveBeginPlay`
  (`parent.ReceiveBeginPlay`))

(event `self.ReceiveTick`
  (params (DeltaSeconds :type "Float (single-precision)"))
  (`parent.ReceiveTick` DeltaSeconds))

(event `Behavior Loop`
  ;[0 0 0] Behavior Loop - Animation Flipbook
  (if (`self.Is Finished`)
    (set `self.Is Finished` false)
    (`self.Ramdom Value Setting`)
    (`self.Behavior Loop`)
    (elif (<= (`self.Behavior Value`) 5.0)
      (`PaperFlipbookComponent.SetFlipbook` (`self.Sprite`) "/Game/PaperAssets/Characters/Neutral/Flipbook/Cat_Black_Idle.Cat_Black_Idle")
      (`self.Behavior Loop`)
      (elif (<= (`self.Behavior Value`) 6.5)
        (`PaperFlipbookComponent.SetFlipbook` (`self.Sprite`) "/Game/PaperAssets/Characters/Neutral/Flipbook/Cat_Black_Meow.Cat_Black_Meow")
        (`self.Behavior Loop`)
        (elif (<= (`self.Behavior Value`) 8.0)
          (`PaperFlipbookComponent.SetFlipbook` (`self.Sprite`) "/Game/PaperAssets/Characters/Neutral/Flipbook/Cat_Black_Stretch.Cat_Black_Stretch")
          (`self.Behavior Loop`)
          (else
            (set `self.Is Walking` true)
            (`self.Behavior Loop`)))))))

(event `Move Forward`
  (params (ScaleValue :type "Float (single-precision)"))
  ;[0 0 0] Move Forward
  (`self.AddMovementInput` (`self.GetActorForwardVector`) ScaleValue))

(event `self.Wall Detector.OnComponentBeginOverlap`
  (params (OverlappedComponent :type "PrimitiveComponent Object Reference") (OtherActor :type "Actor Object Reference") (OtherComp :type "PrimitiveComponent Object Reference") (OtherBodyIndex :type Integer) (bFromSweep :type Boolean) (SweepResult :type "HitResult Structure (by ref)"))
  ;[0 0 0] Wall Detector : Turn Character
  (`self.Trun Character`))

(event `Ramdom Value Setting`
  ;[0 0 0] Random Value Setting
  (set `self.Behavior Value` (`KismetMathLibrary.RandomFloatInRange` 0.0 10.0)))

(fn `UserConstructionScript`
  (`parent.UserConstructionScript`))