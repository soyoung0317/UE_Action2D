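; Bat enemy that patrols back and forth between two points marked by its TopPos and BottomPos components.
; BeginPlay caches both world positions, so they stay fixed as the actor moves, and applies a configurable play rate to the MoveAnim timeline.
; The timeline lerps actor location without sweep, and a FlipFlop on Finished alternates reverse and forward playback to loop endlessly without Tick.
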(event `self.ReceiveBeginPlay`
  (`parent.ReceiveBeginPlay`)
  (set `self.World TopPos` (`SceneComponent.K2_GetComponentLocation` (`self.TopPos`))) ; 변수화
  (set `self.World BottomPos` (`SceneComponent.K2_GetComponentLocation` (`self.BottomPos`))) ; 변수화
  (`TimelineComponent.SetPlayRate` (`self.moveAnim`) (`self.Move PlayRate`)) ; 몬스터마다 설정을 변수화 하여 다르게
  (`self.Move Foward`))

(event `Move Foward`
  (bind (_direction _alpha) (`Timeline|moveAnim` :!via `PlayFromStart` :!label _label)
    (:`Update`
      (`self.K2_SetActorLocation` (`KismetMathLibrary.VLerp` (`self.World TopPos`) (`self.World BottomPos`) _alpha)))
    (:`Finished`
      (`/Engine/EditorBlueprintResources/StandardMacros.FlipFlop`
        (:`A`
          (`self.Move Backward`))
        (:`B`
          (`self.Move Foward`))))))

(event `Move Backward`
  (goto _label :!via `ReverseFromEnd`))

(fn `UserConstructionScript`
  (`parent.UserConstructionScript`))