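; BP_Enemy_BASE is a base Blueprint for enemy characters, handling their defeat and removal from the game.
; On BeginPlay it binds OnDefeated to the Defeated event dispatcher, which destroys the actor when fired.
; The Destroyed override spawns BP_VFX_EnemyDestroyed at the actor's location and rotation, so the effect accompanies its removal.
; A TurnCharacter helper flips the actor 180 degrees by combining rotators.
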(event `self.ReceiveBeginPlay`
  ;[0 0 0] Event Dispatchers Listening
  (`parent.ReceiveBeginPlay`)
  (add `self.Defeated` (delegate `OnDefeated`)))

(event `OnDefeated`
  ;[0 0 0] Event Dispatchers Listening
  (`self.K2_DestroyActor`))

(event `self.ReceiveDestroyed`
  ;[0 0 0] (Override) Event Destroyed : 삭제될 때 객체 위치에서 VFX 생성하기
  (`|SpawnActorFromClass` "/Game/Blueprints/VFX/BP_VFX_EnemyDestroyed.BP_VFX_EnemyDestroyed_C" (`KismetMathLibrary.MakeTransform` (`self.K2_GetActorLocation`) (`self.K2_GetActorRotation`)) "AlwaysSpawn" "MultiplyWithRoot" null null))

(fn `Turn Character`
  ;[0 0 0] 180도 뒤집기
  (`self.K2_SetActorRotation` (`KismetMathLibrary.ComposeRotators` (`self.K2_GetActorRotation`) (struct :`Yaw` 180.0))))

(fn `UserConstructionScript`
  (`parent.UserConstructionScript`))