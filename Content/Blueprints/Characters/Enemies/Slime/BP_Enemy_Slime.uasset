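; Slime enemy Blueprint that detects the player and moves as directed, with targeting delegated to its AIC_Slime controller.
; PlayerDetector overlaps pass the player to the controller's TargetSetting, and end overlap calls it empty to clear the target.
; MoveTo adds movement input and flips the actor 180 degrees by the sign of X direction.
; A LookAtPlayer function, uncalled here, applies only the roll of a look-at rotation.
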(event `self.Player Detector.OnComponentBeginOverlap`
  (params (OverlappedComponent :type "PrimitiveComponent Object Reference") (OtherActor :type "Actor Object Reference") (OtherComp :type "PrimitiveComponent Object Reference") (OtherBodyIndex :type Integer) (bFromSweep :type Boolean) (SweepResult :type "HitResult Structure (by ref)"))
  ;[0 0 0] Collider에 overlap된 Player&를 AIC에게 보내기
  (bind _asbp_player (cast `/Game/Blueprints/Characters/Player/BP_Player` OtherActor))
  (bind _asaic_slime (cast `/Game/Blueprints/AI/AIC_Slime` (`AIBlueprintHelperLibrary.GetAIController` self)))
  (`/Game/Blueprints/AI/AIC_Slime.Target Setting` _asaic_slime _asbp_player))

(event `self.Player Detector.OnComponentEndOverlap`
  (params (OverlappedComponent :type "PrimitiveComponent Object Reference") (OtherActor :type "Actor Object Reference") (OtherComp :type "PrimitiveComponent Object Reference") (OtherBodyIndex :type Integer))
  ;[0 0 0] 플레이어 놓침
  (cast `/Game/Blueprints/Characters/Player/BP_Player` OtherActor)
  (bind _asaic_slime (cast `/Game/Blueprints/AI/AIC_Slime` (`AIBlueprintHelperLibrary.GetAIController` self)))
  (`/Game/Blueprints/AI/AIC_Slime.Target Setting` _asaic_slime null))

(event `self.ReceiveTick`
  (params (DeltaSeconds :type "Float (single-precision)"))
  (`parent.ReceiveTick` DeltaSeconds))

(event `Move To`
  (params (`World Direction` :type "Vector Structure") (Scale :type "Float (double-precision)" :default 1.0))
  ;[0 0 0] 움직여야하는 Direction의 x가 반대편일경우 해당 방향으로 회전하는 함수
  (`self.AddMovementInput` `World Direction` Scale)
  (`self.K2_SetActorRotation` (select `bool` (< (.x `World Direction`) 0.0) :`true` (struct :`Yaw` 180.0) :!type "Rotator Structure")))

(fn `LookAt Player`
  (bind _returnvalue_roll (`KismetMathLibrary.BreakRotator` (`KismetMathLibrary.FindLookAtRotation` (`self.K2_GetActorLocation`) (`self.K2_GetActorLocation`))))
  (`/Engine/EditorBlueprintResources/StandardMacros.IsValid` null
    (:`Is Valid`
      (`self.K2_SetActorRotation` (`KismetMathLibrary.MakeRotator` _returnvalue_roll)))))

(fn `UserConstructionScript`
  (`parent.UserConstructionScript`))