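; BP_Enemy_Crab is a flipbook-animated crab enemy that patrols, turning around at walls and ledges.
; A WalkFoward event moves it along its forward vector, while wall-detector begin overlaps and ledge-detector end overlaps call TurnCharacter.
; Tick switches between idle and walk flipbooks by velocity and plays footstep sounds on two walk frames, using a DoOnce to avoid repeats.
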(event `self.ReceiveTick`
  (params (DeltaSeconds :type "Float (single-precision)"))
  (bind _returnvalue (`PaperFlipbookComponent.GetPlaybackPositionInFrames` (`self.Sprite`)))
  ;[0 0 0] Comment
  (`parent.ReceiveTick` DeltaSeconds)
  (`self.Update Animation`)
  (if (== (`PaperFlipbookComponent.GetFlipbook` (`self.Sprite`)) "/Game/PaperAssets/Characters/Enemies/crab/crab__Walk.crab__Walk")
    (if (or (== _returnvalue 2) (== _returnvalue 4))
      (`/Engine/EditorBlueprintResources/StandardMacros.DoOnce` false :!label _label
        (:`Completed`
          (`GameplayStatics.PlaySoundAtLocation` "/Game/Audio/SFX/Footstep_Crab_Cue.Footstep_Crab_Cue" (`self.K2_GetActorLocation`) (struct) 1.0 1.0 0.0 null null null null)))
      (else
        (goto _label :!via `Reset`)))))

(event `Walk Foward`
  (params (ScaleValue :type "Float (single-precision)"))
  ;[0 0 0] Movement : Look 방향으로 이동
  (`self.AddMovementInput` (`self.GetActorForwardVector`) ScaleValue))

(event `self.Wall Detector.OnComponentBeginOverlap`
  (params (OverlappedComponent :type "PrimitiveComponent Object Reference") (OtherActor :type "Actor Object Reference") (OtherComp :type "PrimitiveComponent Object Reference") (OtherBodyIndex :type Integer) (bFromSweep :type Boolean) (SweepResult :type "HitResult Structure (by ref)"))
  ;[0 0 0] Wall Detector : 벽 만나면 뒤돌아가기
  (`self.Turn Character`))

(event `self.Ledge Detector.OnComponentEndOverlap`
  (params (OverlappedComponent :type "PrimitiveComponent Object Reference") (OtherActor :type "Actor Object Reference") (OtherComp :type "PrimitiveComponent Object Reference") (OtherBodyIndex :type Integer))
  ;[0 0 0] Ledge Detector : 길이 끊기면 뒤돌아가기
  (`self.Turn Character`))

(fn `Update Animation`
  (`PaperFlipbookComponent.SetFlipbook` (`self.Sprite`) (select `bool` (> (`KismetMathLibrary.VSize` (`self.GetVelocity`)) 0.0) :`false` "/Game/PaperAssets/Characters/Enemies/crab/crab__Idle.crab__Idle" :`true` "/Game/PaperAssets/Characters/Enemies/crab/crab__Walk.crab__Walk" :!type "PaperFlipbook Object Reference")))

(fn `UserConstructionScript`
  (`parent.UserConstructionScript`))