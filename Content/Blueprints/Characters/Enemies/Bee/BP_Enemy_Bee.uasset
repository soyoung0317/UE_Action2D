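; Bee enemy character that patrols, chases the player and returns to its spawn point.
; Trigger overlaps set chase and return flags, passing the detected player to AIC_Bee.
; Exposed events move it: patrol follows NextLocation, whose graph holds a sine-based figure-eight around the start, and chase uses movement input, both flipping to face travel.
; Return hides it behind a sparkle effect, teleporting it home when that effect is destroyed.
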(event `self.ReceiveBeginPlay`
  ;[0 0 0] Begin Play : 변수화 -> 타임라인 연결
  (`parent.ReceiveBeginPlay`)
  (set `self.Start Pos` (`self.K2_GetActorLocation` self)))

(event `self.ReceiveTick`
  (params (DeltaSeconds :type "Float (single-precision)"))
  (`parent.ReceiveTick` DeltaSeconds))

(event `Move Patrol`
  (bind _returnvalue (* (`KismetMathLibrary.Sin` (* (`KismetSystemLibrary.GetGameTimeInSeconds`) (`self.Patrol Speed`))) (`self.Radius`)))
  (bind _returnvalue_2 (+ (`self.Start Pos`) (`KismetMathLibrary.MakeVector` _returnvalue 0.0 (* _returnvalue (`KismetMathLibrary.Cos` (* (`KismetSystemLibrary.GetGameTimeInSeconds`) (`self.Patrol Speed`)))))))
  (bind _returnvalue_x (`KismetMathLibrary.BreakVector` (- (`self.K2_GetActorLocation`) _returnvalue_2)))
  ;[0 0 0] Patrol
  (set `self.Is Returning` false)
  (`self.K2_SetActorRotation` (`KismetMathLibrary.SelectRotator` (struct :`Yaw` 180.0) (struct) (>= _returnvalue_x 0.0)))
  (`self.K2_SetActorLocation` _returnvalue_2))

(event `Move Toward`
  (params (`Move Direction` :type "Vector Structure"))
  ;[0 0 0] Move Toward : 플레이어 포착시 따라가는 함수
  (`self.AddMovementInput` `Move Direction` (`self.Chasing Speed`))
  (`self.K2_SetActorRotation` (`KismetMathLibrary.SelectRotator` (struct :`Yaw` 180.0) (struct) (< (.x `Move Direction`) 0.0))))

(event `Move To Return`
  ;[0 0 0] Return to Spawning Position
  (`|ExecutionSequence`
    (:`then_0`
      (`/Engine/EditorBlueprintResources/StandardMacros.DoOnce` false :!label _label ; 이벤트를 한번 다 돌아야지 리셋함
        (:`Completed`
          (`self.SetActorHiddenInGame` self true)
          (bind _returnvalue (`|SpawnActorFromClass` "/Game/Blueprints/Effect/BP_Effect_Sparkle_1.BP_Effect_Sparkle_1_C" (`KismetMathLibrary.MakeTransform` (`self.K2_GetActorLocation`) (`self.K2_GetActorRotation`)) "AlwaysSpawn" "MultiplyWithRoot" null null))
          (set `self.Teleport Effect` _returnvalue))))
    (:`then_1`
      (`/Engine/EditorBlueprintResources/StandardMacros.IsValid` (`self.Teleport Effect`)
        (:`Is Valid`
          (add `self.OnDestroyed` (`self.Teleport Effect`) (delegate `Effect Destroyed`)))))))

(event `Effect Destroyed` :!signature `self.OnDestroyed`
  (params (DestroyedActor :type "Actor Object Reference"))
  ;[0 0 0] Return to Spawning Position
  (`self.K2_SetActorLocation` (`self.Start Pos`))
  (`self.SetActorHiddenInGame` false)
  (set `self.Is Returning` false)
  (goto _label :!via `Reset`))

(event `self.Trigger.OnComponentBeginOverlap`
  (params (OverlappedComponent :type "PrimitiveComponent Object Reference") (OtherActor :type "Actor Object Reference") (OtherComp :type "PrimitiveComponent Object Reference") (OtherBodyIndex :type Integer) (bFromSweep :type Boolean) (SweepResult :type "HitResult Structure (by ref)"))
  ;[0 0 0] Overlap w.Player -> AIC에게 정보넘김
  (bind _asbp_player (cast `/Game/Blueprints/Characters/Player/BP_Player` OtherActor))
  (bind _output_get (set `self.Target Player` _asbp_player))
  (set `self.Is Chasing` true)
  (set `self.Is Returning` false)
  (bind _asaic_bee (cast `/Game/Blueprints/AI/Monster/AIC_Bee` (`AIBlueprintHelperLibrary.GetAIController` self)))
  (`/Game/Blueprints/AI/Monster/AIC_Bee.Set Target Player` _asaic_bee _output_get))

(event `self.Trigger.OnComponentEndOverlap`
  (params (OverlappedComponent :type "PrimitiveComponent Object Reference") (OtherActor :type "Actor Object Reference") (OtherComp :type "PrimitiveComponent Object Reference") (OtherBodyIndex :type Integer))
  ;[0 0 0] End Overlap -> AIC가 플레이어 잃어버림 + 원래자리 복귀
  (cast `/Game/Blueprints/Characters/Player/BP_Player` OtherActor)
  (set `self.Is Chasing` false)
  (set `self.Is Returning` true))

(fn `UserConstructionScript`
  (`parent.UserConstructionScript`))