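; Arrow trap that repeatedly fires BP_Trap_Projectile actors from its ArrowPos point, using an object pool.
; BeginPlay pre-spawns the pool of projectiles in inactive mode.
; Tick runs a cooldown that sets animation start/end flags each cycle.
; When the spawn-ready flag, which is raised outside this graph, is true, it activates the first idle pooled projectile at ArrowPos and clears the flag.
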(event `self.ReceiveBeginPlay`
  (bind _arrowpos (`self.ArrowPos`))
  ;[0 0 0] Begin Play : Object Pooling을 위해 array 준비 및 셋팅
  (`parent.ReceiveBeginPlay`)
  (for _ (range (+ (`self.Pool Size`) 1))
    (bind _returnvalue (`|SpawnActorFromClass` "/Game/Blueprints/Projectiles/Enemy/BP_Trap_Projectile.BP_Trap_Projectile_C" (`KismetMathLibrary.MakeTransform` (`SceneComponent.K2_GetComponentLocation` _arrowpos) (`SceneComponent.K2_GetComponentRotation` _arrowpos)) "AlwaysSpawn" "MultiplyWithRoot" null null))
    (`/Game/Blueprints/Projectiles/Enemy/BP_Trap_Projectile.Set Inactive Mode` _returnvalue)
    (`KismetArrayLibrary.Array_Add` (`self.arr_Projectiles_Pool`) _returnvalue)))

(event `self.ReceiveTick`
  (params (DeltaSeconds :type "Float (single-precision)"))
  ;[0 0 0] Tick : Cooldown이 되면 arrow를 계속해서 respawn한다.
  (`parent.ReceiveTick` DeltaSeconds)
  (if (`self.b_Is SpawnReady`)
    (`self.Arrow Fire`)
    (set `self.b_Is SpawnReady` false)
    (else
      (bind _output_get (set `self.m_fAcctime` (+ (`self.m_fAcctime`) (`GameplayStatics.GetWorldDeltaSeconds`))))
      (if (>= _output_get (`self.m_fCycletime`))
        (set `self.m_fAcctime` 0.0)
        (set `self.b_Is AnimEnd` false)
        (set `self.b_Is AnimStart` true)))))

(event `Arrow Fire`
  (bind _arrowpos (`self.ArrowPos`))
  ;[0 0 0] Object Pooling 본문
  (for _array_element (`self.arr_Projectiles_Pool`)
    (`/Engine/EditorBlueprintResources/StandardMacros.IsValid` _array_element
      (:`Is Valid`
        (if (not (`/Game/Blueprints/Projectiles/Enemy/BP_Trap_Projectile.Is Active` _array_element))
          (`/Game/Blueprints/Projectiles/Enemy/BP_Trap_Projectile.Set Active Mode` _array_element (`SceneComponent.K2_GetComponentLocation` _arrowpos) (`SceneComponent.K2_GetComponentRotation` _arrowpos))
          (break))))))

(fn `Cooltime Timer`
  (bind _output_get (set `self.m_fAcctime` (+ (`GameplayStatics.GetWorldDeltaSeconds`) (`self.m_fAcctime`))))
  (if (>= _output_get (`self.m_fCycletime`))
    (set `self.m_fAcctime` 0.0)))

(fn `UserConstructionScript`
  (`parent.UserConstructionScript`))