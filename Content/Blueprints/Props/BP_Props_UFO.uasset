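; UFO prop Blueprint that plays a landing cutscene on BeginPlay, ending at its placed location.
; It caches the actor location as the end point, plus waypoints from child scene components.
; Two chained Timelines lerp it from middle-bottom to middle-top, then down to touchdown; the cached start position is unused.
; Capsule collision is disabled during the motion and restored to query and physics on landing.
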(event `self.ReceiveBeginPlay`
  ;[0 0 0] 위치 변수화 -> 이벤트 발생
  (`parent.ReceiveBeginPlay`)
  (set `self.EndPos` (`self.K2_GetActorLocation`)) ; 현재위치를 마지막도착장소로
  (set `self.Start_Pos` (`SceneComponent.K2_GetComponentLocation` (`self.Start_Scene`)))
  (set `self.Middle_Top_Pos` (`SceneComponent.K2_GetComponentLocation` (`self.Mid_Top_Scene`)))
  (set `self.Middle_Bottom_Pos` (`SceneComponent.K2_GetComponentLocation` (`self.Mid_Bot_Scene`)))
  (`self.Start Cutscene`))

(event `Start Cutscene`
  (`PrimitiveComponent.SetCollisionEnabled` (`self.CapsuleComponent`) "NoCollision")
  ;[1 1 1] Comment
  (bind (_direction _newtrack_0) (`Timeline|Timeline_0` :!via `PlayFromStart`)
    (:`Update`
      (`self.K2_SetActorLocation` (`KismetMathLibrary.VLerp` (`self.Middle_Bottom_Pos`) (`self.Middle_Top_Pos`) _newtrack_0)))
    (:`Finished`
      ;[0 0 0] 마지막 툭 착륙
      (bind (_direction_2 _newtrack_0_2) (`Timeline|Timeline` :!via `PlayFromStart`)
        (:`Update`
          (`self.K2_SetActorLocation` (`KismetMathLibrary.VLerp` (`self.Middle_Top_Pos`) (`self.EndPos`) _newtrack_0_2)))
        (:`Finished`
          (`PrimitiveComponent.SetCollisionEnabled` (`self.CapsuleComponent`) "QueryAndPhysics"))))))

(fn `UserConstructionScript`
  (`parent.UserConstructionScript`))