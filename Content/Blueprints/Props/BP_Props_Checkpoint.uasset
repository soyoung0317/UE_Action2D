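; Checkpoint prop that responds to the player pressing E while inside its trigger.
; Trigger overlap events cache the BP_Player reference and set an overlap flag, which Tick polls along with the player's E-pressed state.
; The first press passes a never-reset DoOnce and sets the cached GM_Action game mode's ActiveCheckpoint to None, leaving a self node unconnected.
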(event `self.ReceiveBeginPlay`
  (`parent.ReceiveBeginPlay`)
  (bind _asgm_action (cast `/Game/Blueprints/GM_Action` (`GameplayStatics.GetGameMode`)))
  (set `self.GM Action` _asgm_action))

(event `self.ReceiveTick`
  (params (DeltaSeconds :type "Float (single-precision)"))
  (`parent.ReceiveTick` DeltaSeconds)
  (if (`self.Is Overlap Player`)
    (if (`/Game/Blueprints/Characters/Player/BP_Player.Is Pressed E` (`self.Player Ref`))
      (`/Engine/EditorBlueprintResources/StandardMacros.DoOnce` false
        (:`Completed`
          (set `/Game/Blueprints/GM_Action.ActiveCheckpoint` null (`self.GM Action`)))))))

(event `self.Trigger.OnComponentBeginOverlap`
  (params (OverlappedComponent :type "PrimitiveComponent Object Reference") (OtherActor :type "Actor Object Reference") (OtherComp :type "PrimitiveComponent Object Reference") (OtherBodyIndex :type Integer) (bFromSweep :type Boolean) (SweepResult :type "HitResult Structure (by ref)"))
  (bind _asbp_player (cast `/Game/Blueprints/Characters/Player/BP_Player` OtherActor))
  (set `self.Player Ref` _asbp_player)
  (set `self.Is Overlap Player` true))

(event `self.Trigger.OnComponentEndOverlap`
  (params (OverlappedComponent :type "PrimitiveComponent Object Reference") (OtherActor :type "Actor Object Reference") (OtherComp :type "PrimitiveComponent Object Reference") (OtherBodyIndex :type Integer))
  (cast `/Game/Blueprints/Characters/Player/BP_Player` OtherActor)
  (set `self.Is Overlap Player` false))

(fn `UserConstructionScript`
  (`parent.UserConstructionScript`))