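; BP_Checkpoint is a 2D checkpoint that the player activates with E inside its trigger, registering itself as GM_Action's active checkpoint.
; On BeginPlay it spawns three star effects at staggered playback rates.
; Tick polls overlap and the player's E flag, consuming the press once.
; After activation, while overlap lasts, Tick plays the LaunchFlag timeline, which lifts the flipbook and destroys the stars.
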(event `self.ReceiveBeginPlay`
  (bind _scene (`self.Scene`))
  (bind _scene1 (`self.Scene1`))
  (bind _scene2 (`self.Scene2`))
  (bind _asgm_action (cast `/Game/Blueprints/GM_Action` (`GameplayStatics.GetGameMode`)))
  (set `self.GM_Action` _asgm_action)
  (bind _returnvalue (`|SpawnActorFromClass` "/Game/Blueprints/Effect/BP_Effect_Star.BP_Effect_Star_C" (`KismetMathLibrary.MakeTransform` (`SceneComponent.K2_GetComponentLocation` _scene) (`SceneComponent.K2_GetComponentRotation` _scene) (0.5 0.5 0.5)) "AlwaysSpawn" "MultiplyWithRoot" null null))
  (bind _output_get (set `self.NewVar` _returnvalue))
  (`PaperFlipbookComponent.SetPlayRate` (`/Game/Blueprints/Effect/BP_Effect_BASE.PaperFlipbook` _output_get) 1.0)
  (bind _returnvalue_2 (`|SpawnActorFromClass` "/Game/Blueprints/Effect/BP_Effect_Star.BP_Effect_Star_C" (`KismetMathLibrary.MakeTransform` (`SceneComponent.K2_GetComponentLocation` _scene1) (`SceneComponent.K2_GetComponentRotation` _scene1) (0.5 0.5 0.5)) "AlwaysSpawn" "MultiplyWithRoot" null null))
  (bind _output_get_2 (set `self.NewVar_0` _returnvalue_2))
  (`PaperFlipbookComponent.SetPlayRate` (`/Game/Blueprints/Effect/BP_Effect_BASE.PaperFlipbook` _output_get_2) 0.8)
  (bind _returnvalue_3 (`|SpawnActorFromClass` "/Game/Blueprints/Effect/BP_Effect_Star.BP_Effect_Star_C" (`KismetMathLibrary.MakeTransform` (`SceneComponent.K2_GetComponentLocation` _scene2) (`SceneComponent.K2_GetComponentRotation` _scene2) (0.5 0.5 0.5)) "AlwaysSpawn" "MultiplyWithRoot" null null))
  (bind _output_get_3 (set `self.NewVar_1` _returnvalue_3))
  (`PaperFlipbookComponent.SetPlayRate` (`/Game/Blueprints/Effect/BP_Effect_BASE.PaperFlipbook` _output_get_3) 0.9))

(event `self.ReceiveTick`
  (params (DeltaSeconds :type "Float (single-precision)"))
  (bind (_returnvalue_x _returnvalue_y _returnvalue_z) (`KismetMathLibrary.BreakVector` (`SceneComponent.K2_GetComponentLocation` (`self.PaperFlipbook`))))
  (if (`self.Is Overlap Player`)
    (if (`/Game/Blueprints/Characters/Player/BP_Player.Is Pressed E` (`self.As BP Player`))
      (`/Engine/EditorBlueprintResources/StandardMacros.DoOnce` false
        (:`Completed`
          (set `/Game/Blueprints/Characters/Player/BP_Player.Is Pressed E` false (`self.As BP Player`))
          (set `/Game/Blueprints/GM_Action.ActiveCheckpoint` self (`self.GM_Action`))
          (set `self.Is New Checkpoint` true)))
      (elif (`self.Is New Checkpoint`)
        (bind (_direction _alpha) (`Timeline|Launch Flag`)
          (:`Update`
            (`SceneComponent.K2_SetWorldLocation` (`self.PaperFlipbook`) (`KismetMathLibrary.MakeVector` _returnvalue_x _returnvalue_y (+ _returnvalue_z (* _alpha 8.0))) false false)
            (`/Engine/EditorBlueprintResources/StandardMacros.DoOnce` false
              (:`Completed`
                (`self.K2_DestroyActor` (`self.NewVar`))
                (`self.K2_DestroyActor` (`self.NewVar_0`))
                (`self.K2_DestroyActor` (`self.NewVar_1`)))))
          (:`Finished`
            (`self.SetActorHiddenInGame` false)))))))

(event `self.Trigger.OnComponentBeginOverlap`
  (params (OverlappedComponent :type "PrimitiveComponent Object Reference") (OtherActor :type "Actor Object Reference") (OtherComp :type "PrimitiveComponent Object Reference") (OtherBodyIndex :type Integer) (bFromSweep :type Boolean) (SweepResult :type "HitResult Structure (by ref)"))
  (bind _asbp_player (cast `/Game/Blueprints/Characters/Player/BP_Player` OtherActor))
  (set `self.As BP Player` _asbp_player)
  (set `self.Is Overlap Player` true))

(event `self.Trigger.OnComponentEndOverlap`
  (params (OverlappedComponent :type "PrimitiveComponent Object Reference") (OtherActor :type "Actor Object Reference") (OtherComp :type "PrimitiveComponent Object Reference") (OtherBodyIndex :type Integer))
  (bind _asbp_player (cast `/Game/Blueprints/Characters/Player/BP_Player` OtherActor))
  (set `self.As BP Player` _asbp_player)
  (set `self.Is Overlap Player` false))

(fn `UserConstructionScript`)