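; BP_CameraRestrictor is a trigger actor that restricts the player's camera while BP_Player overlaps it.
; On begin overlap it registers itself on the player and, if IsSettingLength is set, passes SetArmLength to ControlOrthoCameraSetting as the new ortho width.
; On end overlap it clears that reference and always calls the same function with OriginArmLength and the IsSettingLength flag.
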(event `self.Trigger.OnComponentBeginOverlap`
  (params (OverlappedComponent :type "PrimitiveComponent Object Reference") (OtherActor :type "Actor Object Reference") (OtherComp :type "PrimitiveComponent Object Reference") (OtherBodyIndex :type Integer) (bFromSweep :type Boolean) (SweepResult :type "HitResult Structure (by ref)"))
  (bind _asbp_player (cast `/Game/Blueprints/Characters/Player/BP_Player` OtherActor))
  (set `/Game/Blueprints/Characters/Player/BP_Player.Camera OverapRistrictor` self _asbp_player)
  (if (`self.Is Setting Length`)
    (`/Game/Blueprints/Characters/Player/BP_Player.Control OrthoCamera Setting` _asbp_player (`self.Is Setting Length`) (`self.Set ArmLength`))))

(event `self.Trigger.OnComponentEndOverlap`
  (params (OverlappedComponent :type "PrimitiveComponent Object Reference") (OtherActor :type "Actor Object Reference") (OtherComp :type "PrimitiveComponent Object Reference") (OtherBodyIndex :type Integer))
  ;[0 0 0] Comment
  (bind _asbp_player (cast `/Game/Blueprints/Characters/Player/BP_Player` OtherActor))
  (set `/Game/Blueprints/Characters/Player/BP_Player.Camera OverapRistrictor` null _asbp_player)
  (`/Game/Blueprints/Characters/Player/BP_Player.Control OrthoCamera Setting` _asbp_player (`self.Is Setting Length`) (`self.Origin ArmLength`)))

(fn `UserConstructionScript`)