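; Pooled Paper2D enemy trap projectile that toggles between active and inactive states instead of being destroyed.
; SetActiveMode places it, re-enables flipbook and collision, and launches it at fixed speed along world ±X, chosen by the forward vector's X sign.
; On sphere hit it spawns hit VFX, then SetInactiveMode stops, hides and parks it at the origin without collision.
; A separate HitEffect function, uncalled here, adds a destruction sound to the VFX.
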(event `self.ReceiveBeginPlay`
  (`parent.ReceiveBeginPlay`))

(event `self.Sphere.OnComponentHit`
  (params (HitComponent :type "PrimitiveComponent Object Reference") (OtherActor :type "Actor Object Reference") (OtherComp :type "PrimitiveComponent Object Reference") (NormalImpulse :type "Vector Structure") (Hit :type "HitResult Structure (by ref)"))
  (bind _sphere (`self.Sphere`))
  ;[0 0 0] Object Pooling Retrieve
  (`|SpawnActorFromClass` "/Game/Blueprints/VFX/BP_VFX_ShotHit.BP_VFX_ShotHit_C" (`KismetMathLibrary.MakeTransform` (`SceneComponent.K2_GetComponentLocation` _sphere) (`SceneComponent.K2_GetComponentRotation` _sphere)) "AlwaysSpawn" "MultiplyWithRoot" null null)
  (`self.Set Inactive Mode`))

(event `self.ReceiveTick`
  (params (DeltaSeconds :type "Float (single-precision)"))
  (`parent.ReceiveTick` DeltaSeconds))

(event `Set Inactive Mode`
  ;[0 0 0] 비활성화 모드로 전환
  (`self.K2_SetActorLocation` (0.0 0.0 0.0))
  (set `MovementComponent.Velocity` (0.0 0.0 0.0) (`self.ProjectileMovement`))
  (set `self.Is Active` false)
  (`SceneComponent.SetHiddenInGame` (`self.PaperFlipbook`) true false)
  (`PrimitiveComponent.SetCollisionEnabled` (`self.Sphere`) "NoCollision"))

(event `Set Active Mode`
  (params (`New Location` :type "Vector Structure") (`New Rotation` :type "Rotator Structure"))
  (bind _returnvalue_x (`KismetMathLibrary.BreakVector` (`self.GetActorForwardVector`)))
  ;[0 0 0] 활성화 모드로 전환
  (`self.K2_SetActorLocation` `New Location`)
  (`self.K2_SetActorRotation` `New Rotation`)
  (`MovementComponent.SetUpdatedComponent` (`self.ProjectileMovement`) (`self.Sphere`))
  (set `MovementComponent.Velocity` (`KismetMathLibrary.SelectVector` (800.0 0.0 0.0) (-800.0 0.0 0.0) (> _returnvalue_x 0.0)) (`self.ProjectileMovement`))
  (set `self.Is Active` true)
  (`SceneComponent.SetHiddenInGame` (`self.PaperFlipbook`) false false)
  (`PrimitiveComponent.SetCollisionEnabled` (`self.Sphere`) "QueryAndPhysics"))

(fn `Hit Effect`
  (`|SpawnActorFromClass` "/Game/Blueprints/VFX/BP_VFX_ShotHit.BP_VFX_ShotHit_C" (`KismetMathLibrary.MakeTransform` (`self.K2_GetActorLocation`) (`self.K2_GetActorRotation`)) "AlwaysSpawn" "MultiplyWithRoot" null null)
  (`GameplayStatics.PlaySoundAtLocation` "/Game/Audio/SFX/Destroyed_Projectile_Cue.Destroyed_Projectile_Cue" (`self.K2_GetActorLocation`) (struct) 1.0 1.0 0.0 null null null null))

(fn `UserConstructionScript`
  (`parent.UserConstructionScript`))