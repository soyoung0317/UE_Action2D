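; Base Blueprint for player projectiles, tied to the player's shot energy.
; On BeginPlay it caches its Owner as the owning BP_Player.
; Each tick it projects its location to screen space and destroys itself past the left or right viewport edge; the vertical axis is not checked.
; When destroyed for any reason, it calls RestoreShotEnergy on the owning player if still valid.
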(event `self.ReceiveBeginPlay`
  ;[0 0 0] Event BeginPlay : 현재 객체의 Owner 설정하기
  (`parent.ReceiveBeginPlay`)
  (bind _asbp_player (cast `/Game/Blueprints/Characters/Player/BP_Player` (`self.GetOwner`)))
  (set `self.OwningPlayer` _asbp_player))

(event `self.ReceiveTick`
  (params (DeltaSeconds :type "Float (single-precision)"))
  (bind _returnvalue_x (`KismetMathLibrary.BreakVector2D` (`WidgetLayoutLibrary.GetViewportSize`)))
  (bind _screenlocation (`PlayerController.ProjectWorldLocationToScreen` (`GameplayStatics.GetPlayerController` 0) (`self.K2_GetActorLocation`) false))
  ;[0 0 0] Event Tick : 매틱마다 뷰포트 밖으로 나간 총알 없애기
  (`parent.ReceiveTick` DeltaSeconds)
  (if (or (<= (`KismetMathLibrary.BreakVector2D` _screenlocation) 0.0) (>= (`KismetMathLibrary.BreakVector2D` _screenlocation) _returnvalue_x))
    (`self.K2_DestroyActor`)))

(event `self.ReceiveDestroyed`
  ;[0 0 0] Event Destoryed : 총알이 삭제될때 슈팅에너지 충전하기
  (`parent.ReceiveDestroyed`)
  (bind _owningplayer (`self.OwningPlayer`)
    (:`then`
      (`/Game/Blueprints/Characters/Player/BP_Player.Restore Shot Energy` _owningplayer))
    (:`else`)))

(fn `UserConstructionScript`
  (`parent.UserConstructionScript`))